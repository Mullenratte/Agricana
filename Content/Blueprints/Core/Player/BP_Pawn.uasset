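; BP_Pawn is a player pawn that provides smooth camera zoom through a spring arm.
; The Zoom axis input adds a scaled offset to DesiredZoom and clamps it to a fixed distance range.
; Tick interpolates the spring arm length toward DesiredZoom with FInterpTo, so zoom changes ease in rather than snap.
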(event `InputAxis|InputAxis_Zoom`
  (params (AxisValue :type "Float (single-precision)"))
  (set `self.DesiredZoom` (`KismetMathLibrary.FClamp` (+ (* AxisValue 30.0) (`self.DesiredZoom`)) 350.0 1000.0)))

(event `self.ReceiveTick`
  (params (DeltaSeconds :type "Float (single-precision)"))
  (bind _springarm (`self.SpringArm`))
  (set `SpringArmComponent.TargetArmLength` (`KismetMathLibrary.FInterpTo` (`SpringArmComponent.TargetArmLength` _springarm) (`self.DesiredZoom`) DeltaSeconds 3.0) _springarm))

(fn `UserConstructionScript`)